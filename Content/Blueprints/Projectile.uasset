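; Projectile is a Paper2D projectile actor that damages enemies on overlap.
; Overlaps with MyCharacter are ignored, while any other actor triggers an ExplodyPuff spawn at the projectile's location and destroys it.
; If that actor is an Enemy, its Damage function first receives DamageAmount.
; The construction script adds a half-scale, slightly offset flipbook component.
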(event `self.ReceiveBeginPlay`)

(event `self.ReceiveActorBeginOverlap`
  (params (OtherActor :type "Actor Object Reference"))
  (cast `/Game/Blueprints/MyCharacter` OtherActor
    (:`CastFailed`
      (bind _asenemy (cast `/Game/Blueprints/Enemies/Enemy` OtherActor)
        (:`then`
          (`/Game/Blueprints/Enemies/Enemy.Damage` _asenemy (`self.DamageAmount`)))
        (:`CastFailed`
          _))
      (`|SpawnActorFromClass` "/Game/Blueprints/ExplodyPuff.ExplodyPuff_C" (`KismetMathLibrary.Conv_VectorToTransform` (`self.K2_GetActorLocation`)))
      (`self.K2_DestroyActor`))))

(fn `UserConstructionScript`
  (`AddComponent|PaperFlipbookComponent_58` :`RelativeTransform` (`KismetMathLibrary.MakeTransform` (-30.0 0.0 5.0) (struct) (0.5 0.5 0.5))))