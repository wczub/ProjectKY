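; Breakable brick for a 2D side-view level that shatters when an airborne Character overlaps it, or a Projectile if CanBeKilledByProjectile is set.
; Breaking spawns four BrickDebris pieces at the corners, launches them up and outward with impulses, tints them to the brick's color, then destroys the brick.
; The construction script snaps the brick to Y=0 and colors its sprite blue if projectile-breakable, otherwise red.
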(event `DestroyThisBrick`
  (`|ExecutionSequence`
    (:`then_0`
      (bind _returnvalue (`|SpawnActorFromClass` "/Game/Blueprints/Level/BrickDebris.BrickDebris_C" (`KismetMathLibrary.MakeTransform` (+ (.location (`self.GetTransform`)) (50.0 0.0 -50.0))) true))
      (set `self.CurrentDebrisPiece` _returnvalue)
      (`PrimitiveComponent.AddImpulse` (`self.CurrentDebrisPiece`) (300.0 0.0 200.0) "None" false)
      (bind _asbrick_debris (cast `/Game/Blueprints/Level/BrickDebris` (`self.CurrentDebrisPiece`) :!label _label))
      (`PaperSpriteComponent.SetSpriteColor` _asbrick_debris (`self.CurrentColor`)))
    (:`then_1`
      (bind _returnvalue_2 (`|SpawnActorFromClass` "/Game/Blueprints/Level/BrickDebris.BrickDebris_C" (`KismetMathLibrary.MakeTransform` (+ (.location (`self.GetTransform`)) (50.0 0.0 50.0))) true))
      (set `self.CurrentDebrisPiece` _returnvalue_2)
      (`PrimitiveComponent.AddImpulse` (`self.CurrentDebrisPiece`) (200.0 0.0 300.0) "None" false)
      (goto _label))
    (:`then_2`
      (bind _returnvalue_3 (`|SpawnActorFromClass` "/Game/Blueprints/Level/BrickDebris.BrickDebris_C" (`KismetMathLibrary.MakeTransform` (+ (.location (`self.GetTransform`)) (-50.0 0.0 50.0))) true))
      (set `self.CurrentDebrisPiece` _returnvalue_3)
      (`PrimitiveComponent.AddImpulse` (`self.CurrentDebrisPiece`) (-200.0 0.0 300.0) "None" false)
      (goto _label))
    (:`then_3`
      (bind _returnvalue_4 (`|SpawnActorFromClass` "/Game/Blueprints/Level/BrickDebris.BrickDebris_C" (`KismetMathLibrary.MakeTransform` (+ (.location (`self.GetTransform`)) (-50.0 0.0 -50.0))) true))
      (set `self.CurrentDebrisPiece` _returnvalue_4)
      (`PrimitiveComponent.AddImpulse` (`self.CurrentDebrisPiece`) (-300.0 0.0 200.0) "None" false)
      (goto _label))
    (:`then_4`
      (`self.K2_DestroyActor`))))

(event `self.ReceiveActorBeginOverlap`
  (params (OtherActor :type "Actor Object Reference"))
  (bind _ascharacter (cast `Character` OtherActor)
    (:`then`
      (if (`NavMovementComponent.IsFalling` (`Pawn.GetMovementComponent` _ascharacter))
        (`self.DestroyThisBrick` :!label _label_2)))
    (:`CastFailed`
      (cast `/Game/Blueprints/Projectile` OtherActor)
      (if (`self.CanBeKilledByProjectile`)
        (goto _label_2)))))

(fn `UserConstructionScript`
  (bind _blocksprite (`self.BlockSprite`))
  (`self.K2_SetActorLocation` (`KismetMathLibrary.MakeVector` (.x (`self.K2_GetActorLocation`)) 0.0 (.z (`self.K2_GetActorLocation`))))
  (if (`self.CanBeKilledByProjectile`)
    (`PaperSpriteComponent.SetSpriteColor` _blocksprite (struct :`B` 1.0 :`A` 1.0))
    (else
      (`PaperSpriteComponent.SetSpriteColor` _blocksprite (struct :`R` 1.0 :`A` 1.0))))
  (set `self.CurrentColor` (`PaperSpriteComponent.SpriteColor` (`self.BlockSprite`))))