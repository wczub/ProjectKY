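; Moving ledge actor whose sprite travels back and forth between a start point and an end point.
; A timeline lerps the sprite's relative location, waits on finishing, then reverses or replays based on direction, with play rate set from MovementRate at BeginPlay.
; The construction script can preview the end point via TestEndPoint, which also snaps the actor's Y to zero.
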(event `self.ReceiveBeginPlay`
  (`TimelineComponent.SetPlayRate` (`self.Timeline_0`) (/ 1.0 (`self.MovementRate`))))

(fn `UserConstructionScript`
  (if (`self.TestEndPoint`)
    (`SceneComponent.K2_SetRelativeLocation` (`self.MovingLedgeSprite`) (`self.EndPoint`) false)
    (`self.K2_SetActorLocation` (`KismetMathLibrary.MakeVector` (.x (`self.K2_GetActorLocation`)) 0.0 (.z (`self.K2_GetActorLocation`))))))